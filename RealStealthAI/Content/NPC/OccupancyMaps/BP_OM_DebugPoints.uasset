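; Debug marker actor for NPC occupancy maps that displays a time-growing Score as floating text and a sphere.
; Each Tick adds delta time to Score up to a cap, writes it to the text, and swaps the sphere material once it passes a threshold.
; The text turns to face the player each frame using the player controller's rotation with a half-turn yaw.
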(event EventBeginPlay)

(event Collision|EventActorBeginOverlap
  (params (OtherActor :type Actor%20Object%20Reference)))

(event EventTick
  (params (DeltaSeconds :type Float%20%28single-precision%29))
  (bind _returnvalue (Game|GetPlayerController 0))
  (bind _textrender (Variables|Default|GetTextRender))
  (bind _sphere (Variables|Default|GetSphere))
  (bind _returnvalue_2 (Transformation|GetActorTransform _returnvalue))
  (Utilities|FlowControl|Sequence
    (:then_0
      (Transformation|SetWorldRotation _textrender (Math|Rotator|MakeRotator (.roll (.rotation _returnvalue_2)) 0.0 (.yaw (.rotation _returnvalue_2))) false false)
      (Transformation|AddLocalRotation _textrender "0.000000,180.000000,0.000000" false false))
    (:then_1
      (bind _output_get (Variables|Default|SetScore (+ DeltaSeconds (Variables|Default|GetScore))))
      (if (>= _output_get 25.0)
        (Variables|Default|SetScore 25.0)))
    (:then_2
      (Rendering|Components|TextRender|SetText (Variables|Default|GetTextRender) (Utilities|Text|ToText(Float) (Variables|Default|GetScore) "HalfToEven"))
      (if (> (Variables|Default|GetScore) 15.0)
        (Rendering|Material|SetMaterial _sphere 0 "/Game/AssetPacks/MC_Sample/Demo/Objects/VendingMachine/M_Vend_Touch.M_Vend_Touch")
        (else
          (Rendering|Material|SetMaterial _sphere 0 "/Game/NPC/Materials/M_Red.M_Red"))))))

(fn ConstructionScript)