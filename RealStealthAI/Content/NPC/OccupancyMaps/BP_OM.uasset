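; BP_OM is an NPC occupancy map actor that fills a box-shaped area with a flat grid of candidate slot positions.
; The construction script caches the Box component's world X/Y bounds and center height.
; On BeginPlay, nested loops step through those bounds by CellSize to populate AvailableSlots.
; Draw then always runs, spawning a BP_OM_DebugPoints actor at every slot to visualize the grid.
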(event Custom|Draw
  (for _array_element (Variables|Default|GetAvailableSlots)
    (Game|SpawnActorfromClass "/Game/NPC/OccupancyMaps/BP_OM_DebugPoints.BP_OM_DebugPoints_C" (Math|Transform|MakeTransform _array_element "0, 0, 0" "1.000000,1.000000,1.000000") "Undefined" "MultiplyWithRoot" 0 0)))

(event EventBeginPlay
  (for _index (range 0 (Math|Float|Truncate (/ (- (Variables|Default|GetMaxX) (Variables|Default|GetMinX)) (Variables|Default|GetCellSize))))
    (for _index_2 (range 0 (Math|Float|Truncate (/ (- (Variables|Default|GetMaxY) (Variables|Default|GetMinY)) (Variables|Default|GetCellSize))))
      (Utilities|Array|Add (Variables|Default|GetAvailableSlots) (Math|Vector|MakeVector (+ (* _index (Variables|Default|GetCellSize)) (Variables|Default|GetMinX)) (+ (* _index_2 (Variables|Default|GetCellSize)) (Variables|Default|GetMinY)) (Variables|Default|GetZ)))))
  (CallFunction|Draw))

(fn ConstructionScript
  (bind _box (Variables|Default|GetBox))
  (bind _returnvalue (Transformation|GetWorldLocation _box))
  (bind _returnvalue_2 (Components|Box|GetScaledBoxExtent _box))
  (Variables|Default|SetMinX (- (.x _returnvalue) (.x _returnvalue_2)))
  (Variables|Default|SetMaxX (+ (.x _returnvalue) (.x _returnvalue_2)))
  (Variables|Default|SetMinY (- (.y _returnvalue) (.y _returnvalue_2)))
  (Variables|Default|SetMaxY (+ (.y _returnvalue) (.y _returnvalue_2)))
  (Variables|Default|SetZ (.z _returnvalue)))