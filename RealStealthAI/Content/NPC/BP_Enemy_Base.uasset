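; Base enemy NPC character that provides a patrol route, speed presets, a kick attack and a stealth-takedown reaction.
; MoveTo snaps it into place, plays the paired victim montage and flags KO on the Base or Smart AI controller's blackboard.
; Attack plays a kick montage, with a looping timer sphere-tracing the leg to hit the player.
; Until KO'd, Tick zeroes the score of OM debug points within OMCone that pass a visibility trace.
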(event Custom|Attack
  (Animation|Montage|PlayMontage (Variables|Character|GetMesh) "/Game/NPC/Animation/H2H_Kick02_Montage.H2H_Kick02_Montage" 1.75
    (:OnCompleted
      _)
    (:OnInterrupted
      _))
  (Default|CallOnAttackEnd))

(event Custom|MoveTo
  (params (Location :type Vector) (Rotation :type Rotator))
  (bind _self self)
  (bind _key_ko_d (Variables|Default|GetKey%20KO'd))
  (bind _returnvalue (AI|GetAIController _self))
  (Pawn|Components|CharacterMovement|DisableMovement (Variables|Character|GetCharacterMovement))
  (Transformation|SetActorTransform _self (Math|Transform|MakeTransform Location Rotation "1.000000,1.000000,1.000000") false true)
  (Animation|PlayAnimMontage "/Game/NPC/Animation/Paired_Knife_Stealth_KidneyAndNeck_Vic_Montage.Paired_Knife_Stealth_KidneyAndNeck_Vic_Montage" 1.0 "None")
  (bind _asaic_npc_base (Utilities|Casting|CastToAIC_NPC_Base _returnvalue)
    (:then
      (AI|Components|Blackboard|SetValueasBool (AI|GetBlackboard _asaic_npc_base) _key_ko_d true)
      (Variables|Default|SetKO true))
    (:CastFailed
      (bind _asaic_npc_smart (Utilities|Casting|CastToAIC_NPC_Smart _returnvalue))
      (AI|Components|Blackboard|SetValueasBool (AI|GetBlackboard _asaic_npc_smart) _key_ko_d true)
      (Variables|Default|SetKO true))))

(event Custom|ScanOM
  (for _array_element (Collision|GetOverlappingActors (Variables|Default|GetOM_Cone) "/Game/NPC/OccupancyMaps/BP_OM_DebugPoints.BP_OM_DebugPoints_C" :!class /Script/Engine.PrimitiveComponent)
    (bind _outhit (Collision|LineTraceByChannel (Transformation|GetWorldLocation (Variables|Character|GetMesh)) (Transformation|GetWorldLocation (Variables|/Script/Engine.Actor|GetRootComponent _array_element)) "TraceTypeQuery1" false 0 "None"))
    (if (not (.bblockinghit _outhit))
      (bind _asbp_om_debug_points (Utilities|Casting|CastToBP_OM_DebugPoints _array_element))
      (Variables|/Game/NPC/OccupancyMaps/BP_OM_DebugPoints.BP_OM_DebugPoints_C|SetScore _asbp_om_debug_points 0.0))))

(event Custom|Trace%20Kick
  (bind _mesh (Variables|Character|GetMesh))
  (bind (_outhit _returnvalue) (Collision|SphereTraceForObjects (.location (Transformation|GetSocketTransform _mesh "thigh_trace" "RTS_World")) (.location (Transformation|GetSocketTransform _mesh "foot_r_trace" "RTS_World")) 25.0 (Utilities|Array|MakeArray "ObjectTypeQuery3") false 0 "ForOneFrame" true "(R=1.000000,G=0.000000,B=0.000000,A=1.000000)" "(R=0.000000,G=1.000000,B=0.000000,A=1.000000)" 0.1))
  (if _returnvalue
    (bind _asbp_player (Utilities|Casting|CastToBP_Player (.HitActor (Collision|BreakHitResult _outhit))))
    (Default|Hit _asbp_player)))

(event EventStartKickTrace
  (bind _returnvalue (Utilities|Time|SetTimerbyEvent (delegate Custom|Trace%20Kick) 0.1 true))
  (Variables|Default|SetKickTraceLoop _returnvalue))

(event EventEndKickTrace
  (bind _kicktraceloop (Variables|Default|GetKickTraceLoop))
  (if (Utilities|Time|IsValidTimerHandle _kicktraceloop)
    (Utilities|Time|ClearandInvalidateTimerbyHandle _kicktraceloop)))

(event EventTick
  (params (DeltaSeconds :type Float%20%28single-precision%29))
  (if (not (Variables|Default|GetKO))
    (CallFunction|ScanOM)))

(fn ConstructionScript)

(fn GetPatrolRoute
  (return (Variables|AI|GetPatrolRoute)))

(fn SetMovementSpeed
  (params (Speed :type E_MovementSpeed%20Enum :default "NewEnumerator0"))
  (bind _output_get (Variables|/Script/Engine.CharacterMovementComponent|SetMaxWalkSpeed (Variables|Character|GetCharacterMovement) (Utilities|Select :Index Speed :NewEnumerator0 0.0 :NewEnumerator1 8e+01 :NewEnumerator2 1.6e+02 :NewEnumerator3 5e+02)))
  (return _output_get))