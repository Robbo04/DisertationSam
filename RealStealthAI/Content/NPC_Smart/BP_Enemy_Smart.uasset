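; Smart enemy NPC character that exposes attack, patrol route and movement speed functions, and can be the victim of a knife stealth takedown.
; Attack plays a kick montage and signals attack end on completion or interruption.
; MoveTo disables movement, teleports to a given transform, plays the paired victim montage, then sets the KO'd blackboard key through its AI controller.
; SetMovementSpeed maps a speed state to max walk speed.
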(event Custom|Attack
  (Animation|Montage|PlayMontage (Variables|Character|GetMesh) "/Game/NPC/Animation/H2H_Kick02_Montage.H2H_Kick02_Montage" 1.5
    (:OnCompleted
      _)
    (:OnInterrupted
      _))
  (Default|CallOnAttackEnd))

(event Custom|MoveTo
  (params (Location :type Vector) (Rotation :type Rotator))
  (bind _self self)
  (Pawn|Components|CharacterMovement|DisableMovement (Variables|Character|GetCharacterMovement))
  (Transformation|SetActorTransform _self (Math|Transform|MakeTransform Location Rotation "1.000000,1.000000,1.000000") false true)
  (Animation|PlayAnimMontage "/Game/NPC/Animation/Paired_Knife_Stealth_KidneyAndNeck_Vic_Montage.Paired_Knife_Stealth_KidneyAndNeck_Vic_Montage" 1.0 "None")
  (bind _asaic_npc_base (Utilities|Casting|CastToAIC_NPC_Base (AI|GetAIController _self)))
  (AI|Components|Blackboard|SetValueasBool (AI|GetBlackboard _asaic_npc_base) (Variables|Default|GetKey%20KO'd) true))

(fn ConstructionScript)

(fn GetPatrolRoute
  (return (Variables|AI|GetPatrolRoute)))

(fn SetMovementSpeed
  (params (Speed :type E_MovementSpeed%20Enum :default "NewEnumerator0"))
  (bind _output_get (Variables|/Script/Engine.CharacterMovementComponent|SetMaxWalkSpeed (Variables|Character|GetCharacterMovement) (Utilities|Select :Index Speed :NewEnumerator0 0.0 :NewEnumerator1 8e+01 :NewEnumerator2 1.6e+02 :NewEnumerator3 5e+02)))
  (return _output_get))