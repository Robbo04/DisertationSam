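; BP_Radio is a radio gameplay object that highlights when the player is in range and can emit noise.
; Its Box overlap events check for BP_Player, swap the Radio mesh to a green material and set Active, reverting both on exit.
; A PlayAudio event calls MakeNoise and plays a sound at world origin, though no sound asset or noise parameters are set.
; Nothing in this graph calls PlayAudio or reads Active.
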(event OnComponentBeginOverlap(Box)
  (params (OverlappedComponent :type Primitive%20Component%20Object%20Reference) (OtherActor :type Actor%20Object%20Reference) (OtherComp :type Primitive%20Component%20Object%20Reference) (OtherBodyIndex :type Integer) (bFromSweep :type Boolean) (SweepResult :type Hit%20Result%20Structure%20%28by%20ref%29))
  (if (Class|GameplayStatics|ObjectIsA OtherActor "/Game/Player/BP_Player.BP_Player_C")
    (Rendering|Material|SetMaterial (Variables|Default|GetRadio) 0 "/Game/NPC/Materials/M_Green.M_Green")
    (Variables|Default|SetActive true)))

(event OnComponentEndOverlap(Box)
  (params (OverlappedComponent :type Primitive%20Component%20Object%20Reference) (OtherActor :type Actor%20Object%20Reference) (OtherComp :type Primitive%20Component%20Object%20Reference) (OtherBodyIndex :type Integer))
  (if (Class|GameplayStatics|ObjectIsA OtherActor "/Game/Player/BP_Player.BP_Player_C")
    (Rendering|Material|SetMaterial (Variables|Default|GetRadio) 0 "/Game/AssetPacks/MC_Sample/Demo/Objects/Props/Prop_Hat/M_Prop_Hat.M_Prop_Hat")
    (Variables|Default|SetActive false)))

(event Custom|PlayAudio
  (Class|Actor|MakeNoise 1.0 0 "0, 0, 0" 0.0 "None")
  (Audio|PlaySoundatLocation 0 "0, 0, 0" "0, 0, 0" 1.0 1.0 0.0 0 0 0 0))

(event EventBeginPlay)

(event Collision|EventActorBeginOverlap
  (params (OtherActor :type Actor%20Object%20Reference)))

(event EventTick
  (params (DeltaSeconds :type Float%20%28single-precision%29)))

(fn ConstructionScript)